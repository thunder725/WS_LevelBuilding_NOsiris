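; BP_Recepteur is a receiver that checks whether inputs arrive in the order defined by IndexArray, as in a sequence puzzle.
; BeginPlay fills a boolean progress array and prints debug values.
; Reception compares each incoming value to the current expected one, flagging it and advancing on a match.
; A mismatch resets the index, but not the flags, and makes every BP_Activator usable again; completion triggers no action here.
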(event Custom|Reception
  (params (i :type Integer))
  (bind _indexarray (Variables|Default|GetindexArray))
  ;[1 0 0.03699] Reception
  (if (< (Variables|Default|GetindexInteraction) (Utilities|Array|Length _indexarray))
    (if (== i (Utilities|Array|Get(acopy) _indexarray (Variables|Default|GetindexInteraction)))
      (Utilities|Array|SetArrayElem (Variables|Default|GetArrayBool) (Variables|Default|GetindexInteraction) true)
      (Variables|Default|SetindexInteraction (+ (Variables|Default|GetindexInteraction) 1))
      (else
        (Variables|Default|SetindexInteraction 0)
        (bind _outactors (Actor|GetAllActorsOfClass "/Game/Game/Blueprint/BP_Activator.BP_Activator_C"))
        (for _array_element _outactors
          (bind _asbp_activator (Utilities|Casting|CastToBP_Activator _array_element))
          (Variables|/Game/Game/Blueprint/BP_Activator.BP_Activator_C|SetUsable _asbp_activator true))))))

(event EventBeginPlay
  ;[1 0 0.963] Creation
  (for _index (range 1 (Utilities|Array|Length (Variables|Default|GetindexArray)))
    (Utilities|Array|Add (Variables|Default|GetArrayBool) (not (Math|Conversions|ToBoolean(Integer) _index)))
    (Development|PrintString (Utilities|String|ToString(Boolean) (Utilities|Array|Get(acopy) (Variables|Default|GetArrayBool) _index)))))

(fn ConstructionScript)

(fn Index++
  (Variables|Default|SetindexInteraction (+ (Variables|Default|GetindexInteraction) 1)))